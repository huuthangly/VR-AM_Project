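; BP_Nozzle animates a 3D printer nozzle, moving its Head component along the printer's X axis, which is Unreal's Y.
; On BeginPlay it calls GenerateData, then fetches segment durations and X positions, storing the positions as target points offset from the Head's starting location.
; Tick linearly interpolates the Head to each target over its duration, skips non-positive durations, prints elapsed time, and stops after the last point.
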(event Custom|BeginMovement
  ;[0.15 0.15 0.15 0.5] Initial Setup for Movement
  (Utilities|FlowControl|Sequence
    (:then_0
      (bind _output_get (Variables|Default|SetCurrentIndex 0)))
    (:then_1
      (Variables|Default|SetMoveTimeElapsed 0.0))
    (:then_2
      (Variables|Default|SetIsMoving true))
    (:then_3
      (Variables|Default|SetCurrentDuration (Utilities|Array|Get(acopy) (Variables|Default|GetDurations) _output_get)))))

(event EventBeginPlay
  ;[0.15 0.15 0.15 0.5] Load Data for Movement
  (CallFunction|GenerateData)
  (bind _returnvalue (CallFunction|GetTime))
  (Variables|Default|SetDurations _returnvalue)
  (bind _returnvalue_2 (CallFunction|GetXPositions))
  (Utilities|FlowControl|Sequence
    (:then_0
      (bind _output_get (Variables|Default|SetStartLocation (Variables|/Script/Engine.SceneComponent|GetRelativeLocation (Variables|Default|GetHead)))))
    (:then_1
      (for _array_element _returnvalue_2
        (Utilities|Array|Add (Variables|Default|GetTargetPoints) (+ _output_get (Math|Vector|MakeVector 0.0 _array_element 0.0))))
      (CallFunction|BeginMovement))))

(event EventTick
  (params (DeltaSeconds :type Float%20%28single-precision%29))
  ;[0.15 0.15 0.15 0.5] Movement in Y direction (UE5) and X direction (3D printer)
  (if (Variables|Default|GetIsMoving)
    (bind _output_get (Variables|Default|SetMoveTimeElapsed (+ DeltaSeconds (Variables|Default|GetMoveTimeElapsed))))
    (Development|PrintText (Utilities|Text|ToText(Float) _output_get "HalfToEven"))
    (if (> (Variables|Default|GetCurrentDuration) 0.0)
      (if (>= (Math|Float|Clamp(Float) (/ _output_get (Variables|Default|GetCurrentDuration))) 0.999)
        (Utilities|FlowControl|Sequence :!label _label
          (:then_0
            (Variables|Default|SetStartLocation (Utilities|Array|Get(acopy) (Variables|Default|GetTargetPoints) (Variables|Default|GetCurrentIndex))))
          (:then_1
            (Variables|Default|SetCurrentIndex (+ (Variables|Default|GetCurrentIndex) 1)))
          (:then_2
            (if (>= (Variables|Default|GetCurrentIndex) (Utilities|Array|Length (Variables|Default|GetTargetPoints)))
              (Development|PrintText "Done")
              (Variables|Default|SetIsMoving false)
              (else
                (Variables|Default|SetMoveTimeElapsed 0.0))))
          (:then_3
            (Variables|Default|SetCurrentDuration (Utilities|Array|Get(acopy) (Variables|Default|GetDurations) (Variables|Default|GetCurrentIndex)))))
        (else
          (Transformation|SetRelativeLocation (Variables|Default|GetHead) (Math|Vector|Lerp(Vector) (Variables|Default|GetStartLocation) (Utilities|Array|Get(acopy) (Variables|Default|GetTargetPoints) (Variables|Default|GetCurrentIndex)) (Math|Float|Clamp(Float) (/ _output_get (Variables|Default|GetCurrentDuration)))) false false)))
      (else
        (goto _label)))))

(fn ConstructionScript)