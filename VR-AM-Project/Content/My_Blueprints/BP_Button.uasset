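; Pressable VR button that starts a print of the file referenced by the print bed.
; VRPawn overlapping the box moves the button down; Tick returns it to its start when its time checks read zero.
; Tick also watches button height, using a DoOnce that re-arms on rise to play a click, call PrintFile and update the printer status text.
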(event OnComponentBeginOverlap(Box)
  (params (OverlappedComponent :type Primitive%20Component%20Object%20Reference) (OtherActor :type Actor%20Object%20Reference) (OtherComp :type Primitive%20Component%20Object%20Reference) (OtherBodyIndex :type Integer) (bFromSweep :type Boolean) (SweepResult :type Hit%20Result%20Structure%20%28by%20ref%29))
  ;[0.15 0.15 0.15 0.5] Push Button Down
  (Utilities|Casting|CastToVRPawn OtherActor)
  (Components|MoveComponentTo (Variables|Default|GetButton) (- (Variables|Default|GetButtonStart) "0.000000,0.000000,5.000000") "0, 0, 0" false false 0.2 false))

(event EventBeginPlay
  ;[0.15 0.15 0.15 0.5] Set Button Start Location
  (Variables|Default|SetButtonStart (Variables|/Script/Engine.SceneComponent|GetRelativeLocation (Variables|Default|GetButton))))

(event EventTick
  (params (DeltaSeconds :type Float%20%28single-precision%29))
  (bind _button (Variables|Default|GetButton))
  (bind _relativelocation (Variables|/Script/Engine.SceneComponent|GetRelativeLocation _button))
  ;[0.15 0.15 0.15 0.5] Set Button Effects
  (Utilities|FlowControl|Sequence
    (:then_0
      ;[0.15 0.15 0.15 0.5] Return Button to Start
      (if (== (Variables|Default|GetTimeBWPressandUpdate) 0)
        (bind _returnvalue (CallFunction|GetTimeValue))
        (if (== _returnvalue 0.0)
          (Components|MoveComponentTo (Variables|Default|GetButton) (Variables|Default|GetButtonStart) "0, 0, 0" false false 0.2 false))))
    (:then_1
      (if (<= (.z _relativelocation) 1.0)
        (Utilities|FlowControl|DoOnce false :!label _label
          (:Completed
            (Utilities|FlowControl|Sequence
              (:then_0
                ;;[0.15 0.15 0.15 0.5] Sound
                (Audio|PlaySoundatLocation "/Game/Level_Assets/Sounds/SC_ButtonClick.SC_ButtonClick" (Transformation|GetWorldLocation (Variables|Default|GetButton)) "0, 0, 0" 1.0 1.0 0.0 0 0 0 0))
              (:then_1
                ;;[0.15 0.15 0.15 0.5] Start to Print
                (bind _outactors (Actor|GetAllActorsOfClass "/Game/My_Blueprints/BP_PrintBed.BP_PrintBed_C"))
                (if (Utilities|IsValid (Variables|/Game/My_Blueprints/BP_PrintBed.BP_PrintBed_C|GetPrintComponentReference (Utilities|Array|Get(acopy) _outactors)))
                  (CallFunction|PrintFile (Variables|/Game/My_Blueprints/PrintComponent.PrintComponent_C|GetFilePath (Variables|/Game/My_Blueprints/BP_PrintBed.BP_PrintBed_C|GetPrintComponentReference (Utilities|Array|Get(acopy) _outactors))))
                  (bind _outactors_2 (Actor|GetAllActorsOfClass "/Game/Level_Assets/Text/Text_Printer_Status.Text_Printer_Status_C"))
                  (Rendering|Components|TextRender|SetText (Variables|/Game/Level_Assets/Text/Text_Printer_Status.Text_Printer_Status_C|GetTextRender (Utilities|Array|Get(acopy) _outactors_2)) (Utilities|Text|ToText(String) (Variables|Default|GetprinterInProgress)))
                  (Rendering|Components|TextRender|SetTextRenderColor (Variables|/Game/Level_Assets/Text/Text_Printer_Status.Text_Printer_Status_C|GetTextRender (Utilities|Array|Get(acopy) _outactors_2)) (Math|Conversions|ToColor(LinearColor) (Math|Color|MakeColor 255.0 255.0 0.0)))
                  (Variables|/Game/Level_Assets/Text/Text_Printer_Status.Text_Printer_Status_C|SetIsUpdated (Utilities|Array|Get(acopy) _outactors_2) (== (- (Variables|Default|GetTimeBWPressandUpdate) 1) 0)))))))
        (elif (>= (.z _relativelocation) 4.0)
          (goto _label Reset))))))

(fn ConstructionScript)