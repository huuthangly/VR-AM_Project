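; BP_PrintBed is a print bed that detects printable objects placed on it and updates the printer's text displays.
; On overlap, it looks for a PrintComponent on the other actor and stores a reference to it.
; It then finds three Text_Printer actors by class to show the component's name with an uploaded message, a green ready status, and a prompt about placing another object.
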(event EventBeginPlay)

(event Collision|EventActorBeginOverlap
  (params (OtherActor :type Actor%20Object%20Reference))
  (bind _returnvalue (Actor|GetComponentbyClass OtherActor "/Game/My_Blueprints/PrintComponent.PrintComponent_C"))
  ;[0.15 0.15 0.15 0.5] Get the File Path and Name when Overlap
  (if (Utilities|IsValid _returnvalue)
    (bind _output_get (Variables|Default|SetPrintComponentReference _returnvalue))
    (Utilities|FlowControl|Sequence
      (:then_0
        (bind _outactors (Actor|GetAllActorsOfClass "/Game/Level_Assets/Text/Text_Printer_CheckObject.Text_Printer_CheckObject_C"))
        (Rendering|Components|TextRender|SetText (Variables|/Game/Level_Assets/Text/Text_Printer_CheckObject.Text_Printer_CheckObject_C|GetTextRender (Utilities|Array|Get(acopy) _outactors)) (Utilities|Text|ToText(String) (Utilities|String|Append (Variables|/Game/My_Blueprints/PrintComponent.PrintComponent_C|GetName _output_get) (Variables|Default|GetisUploaded)))))
      (:then_1
        (bind _outactors_2 (Actor|GetAllActorsOfClass "/Game/Level_Assets/Text/Text_Printer_Status.Text_Printer_Status_C"))
        (Rendering|Components|TextRender|SetText (Variables|/Game/Level_Assets/Text/Text_Printer_Status.Text_Printer_Status_C|GetTextRender (Utilities|Array|Get(acopy) _outactors_2)) (Utilities|Text|ToText(String) (Variables|Default|GetprinterIsReady)))
        (Rendering|Components|TextRender|SetTextRenderColor (Variables|/Game/Level_Assets/Text/Text_Printer_Status.Text_Printer_Status_C|GetTextRender (Utilities|Array|Get(acopy) _outactors_2)) (Math|Color|MakeColor 0 128 0)))
      (:then_2
        (bind _outactors_3 (Actor|GetAllActorsOfClass "/Game/Level_Assets/Text/Text_Printer_PlaceObject.Text_Printer_PlaceObject_C"))
        (Rendering|Components|TextRender|SetText (Variables|/Game/Level_Assets/Text/Text_Printer_PlaceObject.Text_Printer_PlaceObject_C|GetTextRender (Utilities|Array|Get(acopy) _outactors_3)) (Utilities|Text|ToText(String) (Variables|Default|GetplaceAnotherObject)))))))

(fn ConstructionScript)