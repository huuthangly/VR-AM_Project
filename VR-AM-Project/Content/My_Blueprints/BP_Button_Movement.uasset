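; VR push button that moves down and clicks when the VR pawn touches it.
; BeginPlay stores the button's rest position, and a VRPawn overlapping the Box trigger moves the Button component a fixed distance below it.
; Tick polls the button's height to play a click sound once when low, re-arming only above a higher threshold.
; The graph contains no logic to raise the button again.
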(event OnComponentBeginOverlap(Box)
  (params (OverlappedComponent :type Primitive%20Component%20Object%20Reference) (OtherActor :type Actor%20Object%20Reference) (OtherComp :type Primitive%20Component%20Object%20Reference) (OtherBodyIndex :type Integer) (bFromSweep :type Boolean) (SweepResult :type Hit%20Result%20Structure%20%28by%20ref%29))
  ;[0.15 0.15 0.15 0.5] Push Button Down
  (Utilities|Casting|CastToVRPawn OtherActor)
  (Components|MoveComponentTo (Variables|Default|GetButton) (- (Variables|Default|GetButtonStart) "0.000000,0.000000,5.000000") "0, 0, 0" false false 0.2 false))

(event EventBeginPlay
  ;[0.15 0.15 0.15 0.5] Set Button Start Location
  (Variables|Default|SetButtonStart (Variables|/Script/Engine.SceneComponent|GetRelativeLocation (Variables|Default|GetButton))))

(event EventTick
  (params (DeltaSeconds :type Float%20%28single-precision%29))
  (bind _button (Variables|Default|GetButton))
  (bind _relativelocation (Variables|/Script/Engine.SceneComponent|GetRelativeLocation _button))
  ;[0.15 0.15 0.15 0.5] Set Button Effects
  (Utilities|FlowControl|Sequence
    (:then_1
      (if (<= (.z _relativelocation) 1.0)
        (Utilities|FlowControl|DoOnce false :!label _label
          (:Completed
            (Utilities|FlowControl|Sequence
              (:then_0
                ;;[0.15 0.15 0.15 0.5] Sound
                (Audio|PlaySoundatLocation "/Game/Level_Assets/Sounds/SC_ButtonClick.SC_ButtonClick" (Transformation|GetWorldLocation (Variables|Default|GetButton)) "0, 0, 0" 1.0 1.0 0.0 0 0 0 0)))))
        (elif (>= (.z _relativelocation) 4.0)
          (goto _label Reset))))))

(fn ConstructionScript
  (|CallParentFunction))